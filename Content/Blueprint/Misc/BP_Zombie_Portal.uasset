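; BP_Zombie_Portal is a zombie portal actor that turns to face a camera.
; Each tick it gets a reference, checks that it is valid, and computes a look-at rotation toward that object's Camera component.
; It applies only the yaw, keeping pitch and roll at zero so the portal stays upright.
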(event `self.ReceiveBeginPlay`)

(event `self.ReceiveTick`
  (params (DeltaSeconds :type "Float (single-precision)"))
  (bind _returnvalue (`PlayerPawn.Get`))
  (`/Engine/EditorBlueprintResources/StandardMacros.IsValid` _returnvalue
    (:`Is Valid`
      (`self.K2_SetActorRotation` (`KismetMathLibrary.MakeRotator` 0.0 0.0 (.yaw (`KismetMathLibrary.FindLookAtRotation` (`self.K2_GetActorLocation`) (`SceneComponent.K2_GetComponentLocation` (`PlayerPawn.Camera` _returnvalue)))))))))

(fn `UserConstructionScript`)