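; BP_CHaos is an actor that triggers an exploding barrel held in its child actor component after a five-second delay.
; Tick accumulates delta time in a Timer variable until it crosses the threshold, so the trigger fires only once.
; It then casts the child actor to FS_Old_Exploding_Barrel_Blueprint, calls Activate on it and prints a debug message.
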(event `self.ReceiveBeginPlay`)

(event `self.ReceiveTick`
  (params (DeltaSeconds :type "Float (single-precision)"))
  (bind _timer (`self.Timer`))
  (if (< _timer 5.0)
    (bind _output_get (set `self.Timer` (+ _timer DeltaSeconds)))
    (if (>= _output_get 5.0)
      (bind _asfs_old_exploding_barrel_blueprint (cast `/Game/Blueprint/Props/Barrels/FS_Old_Exploding_Barrel_Blueprint` (`ChildActorComponent.ChildActor` (`self.ChildActor`))))
      (`/Game/Blueprint/Props/Barrels/FS_Old_Exploding_Barrel_Blueprint.Activate` _asfs_old_exploding_barrel_blueprint)
      (`KismetSystemLibrary.PrintString` "Enable"))))

(fn `UserConstructionScript`)